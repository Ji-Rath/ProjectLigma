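; Environmental FX actor that spawns a dripping particle emitter at its location and leaves slime drop decals where the particles land.
; On BeginPlay it binds the emitter's particle collision event.
; Each collision creates a dynamic slime decal material with a random frame and spawns a randomly sized, short-lived decal aligned to the hit normal.
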(event Custom|CustomEvent_OnParticleCollide
  (params (EventName :type Name) (EmitterTime :type Float%20%28single-precision%29) (ParticleTime :type Integer) (Location :type Vector) (Velocity :type Vector) (Direction :type Vector) (Normal :type Vector) (BoneName :type Name) (PhysMat :type Physical%20Material%20Object%20Reference))
  (bind _returnvalue (Rendering|Material|CreateDynamicMaterialInstance "/Game/Geometry/Environment/Decals/Blood_slime/Slime_drops.Slime_drops" "None" "None" :!class /Script/Engine.KismetMaterialLibrary))
  (Rendering|Material|SetScalarParameterValue _returnvalue "Frame" (Math|Conversions|ToFloat(Integer) (Math|Random|RandomInteger 11)) :!class /Script/Engine.MaterialInstanceDynamic)
  (Rendering|Decal|SpawnDecalatLocation _returnvalue (Math|Conversions|ToVector(Float) (Math|Random|RandomFloatinRange 1e+01 25.0)) Location (Math|Conversions|RotationFromXVector Normal) 2e+01))

(event EventBeginPlay
  (bind _returnvalue (Effects|SpawnEmitteratLocation "/Game/Geometry/Environment/FX/Drops.Drops" (Transformation|GetActorLocation)))
  (EventDispatchers|BindEventtoOnParticleCollide _returnvalue (delegate Custom|CustomEvent_OnParticleCollide)))

(fn ConstructionScript)