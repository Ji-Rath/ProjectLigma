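; Player controller that swaps control between the starting pawn and a companion BP_Ligma character, and aims at the mouse cursor.
; The Transform input toggles pawns via FlipFlop, spawning Ligma ahead of the player if absent.
; Switches disable input, blend the view, then possess the target after a matching delay; unpossessed pawns stop moving.
; Each tick, a visibility trace under the cursor sets control rotation toward the impact point.
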(event Custom|PossessPawn
  (params (Target :type Pawn%20Object%20Reference))
  (Utilities|IsValid Target
    (:Is%20Valid
      (Game|Player|SetViewTargetwithBlend Target 0.5 "VTBlend_EaseInOut" 2.0 true)
      (Utilities|FlowControl|Delay 0.5)
      (Pawn|Possess Target)
      (Input|EnableInput Target self))))

(event Custom|AlternateCharacters
  (Input|DisableInput (Pawn|GetControlledPawn) self)
  (Utilities|FlowControl|FlipFlop ; Node does not work in functions
    (:A
      (Utilities|IsValid (Variables|Default|GetLigmaRef)
        (:Is%20Valid
          _)
        (:Is%20Not%20Valid
          (CallFunction|SpawnLigma) ; Spawn ligma if not in the world
        ))
      (CallFunction|PossessPawn (Variables|Default|GetOtherPlayerRef)))
    (:B
      (CallFunction|PossessPawn (Variables|Default|GetPlayerRef)))))

(event EventTick
  (params (DeltaSeconds :type Float%20%28single-precision%29))
  (|CallParentFunction DeltaSeconds)
  (CallFunction|LookatMouse))

(event EventBeginPlay
  (|CallParentFunction)
  (Variables|Default|SetPlayerRef (Pawn|GetControlledPawn)))

(event EventUnPossess
  (params (UnpossessedPawn :type Pawn%20Object%20Reference))
  (Utilities|IsValid UnpossessedPawn
    (:Is%20Valid
      (Components|Movement|StopMovementImmediately (Pawn|GetMovementComponent UnpossessedPawn)))))

(event Input|ActionEvents|InputActionTransform
  (params (Key :type Key%20Structure))
  (:Pressed
    (CallFunction|AlternateCharacters)))

(fn ConstructionScript)

(fn SpawnLigma
  (bind _playerref (Variables|Default|GetPlayerRef))
  (bind _returnvalue (Transformation|GetActorTransform _playerref))
  (bind _returnvalue_2 (Game|SpawnActorfromClass "/Game/Blueprints/Player/BP_Ligma.BP_Ligma_C" (Math|Transform|MakeTransform (+ (.location _returnvalue) (* (Transformation|GetActorForwardVector _playerref) 1e+02)) "0, 0, 0" (.scale _returnvalue)) "AdjustIfPossibleButAlwaysSpawn" 0 0))
  (bind _output_get (Variables|Default|SetLigmaRef _returnvalue_2))
  (Variables|Default|SetOtherPlayerRef _output_get))

(fn LookatMouse
  (bind (_worldlocation _worlddirection _returnvalue) (Game|Player|ConvertMouseLocationToWorldSpace))
  (if (and (Utilities|IsValid (Pawn|GetControlledPawn)) _returnvalue)
    (bind _outhit (Collision|LineTraceByChannel _worldlocation (+ _worldlocation (* _worlddirection 5e+03)) "TraceTypeQuery1" false 0 "None"))
    (Pawn|SetControlRotation (Math|Rotator|FindLookatRotation (Transformation|GetActorLocation (Pawn|GetControlledPawn)) (.ImpactPoint (Collision|BreakHitResult _outhit))))))