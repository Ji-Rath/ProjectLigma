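; Player shadow character that possesses or executes enemies whose cast shadow it stands in, and dies in light.
; Each tick, directional-light checks find shadow-casting enemies, a dot product picks the one most faced, and light level sets walk or run speed.
; Possess hides the player and switches pawns; Execute plays synced montages on player, enemy and detached shadow mesh, with camera zoom and ragdolls.
; Lethal light triggers AlternateCharacters, destroying the pawn once unpossessed.
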(event Custom|CheckLightLevel
  (if (>= (Class|LightSenseComponent|GetCurrentLightLevel (Variables|Default|GetLightSense)) 1.0)
    (Variables|Default|SetbPendingDeath true)
    (bind _asbp_player_controller (Utilities|Casting|CastToBP_PlayerController (Pawn|GetController))
      (:then
        (Utilities|FlowControl|DoOnce false ; This node does not work in functions
          (:Completed
            (Default|AlternateCharacters _asbp_player_controller))))
      (:CastFailed
        (Actor|DestroyActor)))))

(event Custom|CameraZoom
  (params (bZoomIn :type Boolean))
  (if bZoomIn
    (bind _camerafocus (Timeline|CameraFocus Play)
      (:Update
        (Variables|/Script/Engine.SpringArmComponent|SetTargetArmLength (Variables|Default|GetSpringArm) (* _camerafocus (Variables|Default|GetSpringArmLength)))))
    (else
      (Timeline|CameraFocus Reverse))))

(event EventTick
  (params (DeltaSeconds :type Float%20%28single-precision%29))
  (|CallParentFunction DeltaSeconds)
  (bind _possessableenemy (CallFunction|GetPossessableEnemies))
  (bind _closestanglepawn (CallFunction|GetLookingatEnemy _possessableenemy))
  (Variables|Default|SetPossessable%20Enemy _closestanglepawn)
  (CallFunction|CheckLightLevel)
  (Variables|/Script/Engine.CharacterMovementComponent|SetMaxWalkSpeed (Variables|Character|GetCharacterMovement) (Math|Float|SelectFloat (Variables|Default|GetWalkSpeed) (Variables|Default|GetRunSpeed) (>= (.ReturnValue (Class|LightSenseComponent|CalculateLightLevel (Transformation|GetActorLocation) (Utilities|Array|MakeArray "/Script/Engine.DirectionalLight") 0 2e+03 false false)) 1.0))))

(event EventUnpossessed
  (params (OldController :type Controller%20Object%20Reference))
  (if (Variables|Default|GetbPendingDeath)
    (Actor|DestroyActor)))

(event EventBeginPlay
  (|CallParentFunction)
  (Variables|Default|SetSpringArmLength (Variables|/Script/Engine.SpringArmComponent|GetTargetArmLength (Variables|Default|GetSpringArm)))
  (Variables|Default|SetWalkSpeed (Variables|/Script/Engine.CharacterMovementComponent|GetMaxWalkSpeed (Variables|Character|GetCharacterMovement))))

(event Input|ActionEvents|InputActionPossess
  (params (Key :type Key%20Structure :default "None"))
  (:Pressed
    (bind _possessable_enemy (Variables|Default|GetPossessable%20Enemy)
      (:then
        (bind _asbp_player_controller (Utilities|Casting|CastToBP_PlayerController (Pawn|GetController)))
        (Default|PossessPawn _asbp_player_controller _possessable_enemy)
        (Rendering|SetActorHiddenInGame true)
        (Variables|/Game/Blueprints/Player/BP_PlayerController.BP_PlayerController_C|SetOtherPlayerRef _asbp_player_controller _possessable_enemy)
        (Transformation|SetActorLocation "0, 0,1000.000000" false false) ; Probably needs a proper location when possessing
      )
      (:else))))

(event Input|ActionEvents|InputActionExecute
  (params (Key :type Key%20Structure :default "None"))
  (:Pressed
    (bind _possessable_enemy (Variables|Default|GetPossessable%20Enemy)
      (:then
        (bind _asbp_enemy_character (Utilities|Casting|CastToBP_EnemyCharacter _possessable_enemy))
        (bind _output_get (Variables|Default|SetEnemyExecute _asbp_enemy_character))
        (CallFunction|CameraZoom true)
        (Transformation|DetachFromComponent (Variables|/Game/Blueprints/AI/BP_EnemyCharacter.BP_EnemyCharacter_C|GetCharacterMesh1 _output_get) "KeepWorld" "KeepRelative" "KeepRelative" true) ; Detach shadow from mesh
        (Collision|SetActorEnableCollision false)
        (CallFunction|GoBehindTarget (Variables|Default|GetEnemyExecute) 1.5e+02)
        (Pawn|Components|CharacterMovement|DisableMovement (Variables|Character|GetCharacterMovement))
        (Animation|Montage|PlayMontage (Variables|/Game/Blueprints/AI/BP_EnemyCharacter.BP_EnemyCharacter_C|GetCharacterMesh1 (Variables|Default|GetEnemyExecute)) "/Game/Mannequin/Animations/Executions/BrutalAssassination_1_4UE4_Montage.BrutalAssassination_1_4UE4_Montage" ; Enemy Shadow Anim
          (:then
            (Animation|Montage|PlayMontage (Variables|/Script/Engine.Character|GetMesh (Variables|Default|GetEnemyExecute)) "/Game/Mannequin/Animations/DizzyIdle4UE4_Montage.DizzyIdle4UE4_Montage" ; Enemy Mesh Dizzy
              (:then
                (Animation|Montage|PlayMontage (Variables|Character|GetMesh) "/Game/Mannequin/Animations/Executions/BrutalAssassination4UE4_Montage.BrutalAssassination4UE4_Montage" ; Player Anim
                  (:OnCompleted
                    (Collision|SetActorEnableCollision true)
                    (Pawn|Components|CharacterMovement|SetMovementMode (Variables|Character|GetCharacterMovement) "MOVE_Walking" 0)
                    (Physics|SetSimulatePhysics (Variables|/Script/Engine.Character|GetMesh (Variables|Default|GetEnemyExecute)) true)
                    (Collision|SetCollisionEnabled (Variables|/Script/Engine.Character|GetCapsuleComponent (Variables|Default|GetEnemyExecute)) "NoCollision"))))))
          (:OnNotifyBegin
            (Physics|SetSimulatePhysics (Variables|/Game/Blueprints/AI/BP_EnemyCharacter.BP_EnemyCharacter_C|GetCharacterMesh1 (Variables|Default|GetEnemyExecute)) true) ; Ragdoll shadow
            (Utilities|IsValid (Pawn|GetController (Variables|Default|GetEnemyExecute))
              (:Is%20Valid
                (Pawn|UnPossess (Pawn|GetController (Variables|Default|GetEnemyExecute))))
              (:Is%20Not%20Valid
                _))
            (CallFunction|CameraZoom false))))
      (:else))))

(fn ConstructionScript)

(fn GetPossessableEnemies
  (bind _outactors (Actor|GetAllActorsOfClass "/Script/Engine.DirectionalLight"))
  (bind _array_element (Utilities|Array|ForEachLoopwithBreak _outactors)
    (:LoopBody
      (bind _array_element_2 (Utilities|Array|ForEachLoopwithBreak (Actor|GetComponentsByClass _array_element "/Script/Engine.DirectionalLightComponent") :!label _label)
        (:LoopBody
          (bind _outactors_2 (Actor|GetAllActorsOfClass "/Game/Blueprints/Player/BP_PlayerBase.BP_PlayerBase_C"))
          (bind _output_get (LocalVariables|SetInShadow (== (.ReturnValue (Class|LightSenseComponent|GetSingleLightLevel _array_element_2 (- (Transformation|GetActorLocation) "0, 0,50.000000") _outactors_2 (Utilities|Array|MakeArray "Flashlight") 2e+03 "ECC_Pawn")) 0.0)))
          (if _output_get
            (LocalVariables|SetPossessableActor (.HitActor (Collision|BreakHitResult (.OutHit (Class|LightSenseComponent|GetSingleLightLevel _array_element_2 (- (Transformation|GetActorLocation) "0, 0,50.000000") _outactors_2 (Utilities|Array|MakeArray "Flashlight") 2e+03 "ECC_Pawn")))))
            (goto _label Break)))
        (:Completed
          (if (LocalVariables|GetInShadow) ; If player is in enemies shadow, add to array
            (bind _asbp_enemy_character (Utilities|Casting|CastToBP_EnemyCharacter (LocalVariables|GetPossessableActor)))
            (Utilities|Array|Add (LocalVariables|GetNearestEnemy) _asbp_enemy_character)))))
    (:Completed
      (return (LocalVariables|GetNearestEnemy)))))

(fn GetLookingatEnemy
  (params (Array :type Array%20of%20Pawn%20Object%20References))
  (bind _array_element (Utilities|Array|ForEachLoopwithBreak Array)
    (:LoopBody
      (if (> (Math|Vector|DotProduct (Math|Vector|GetForwardVector (Math|Rotator|FindLookatRotation (Transformation|GetActorLocation) (Transformation|GetActorLocation _array_element))) (Transformation|GetActorForwardVector)) (LocalVariables|GetDotAngle))
        (LocalVariables|SetClosestPawn _array_element)
        (LocalVariables|SetDotAngle (Math|Vector|DotProduct (Math|Vector|GetForwardVector (Math|Rotator|FindLookatRotation (Transformation|GetActorLocation) (Transformation|GetActorLocation _array_element))) (Transformation|GetActorForwardVector)))))
    (:Completed
      (return (LocalVariables|GetClosestPawn)))))

(fn GoBehindTarget
  (params (EnemyTarget :type Actor%20Object%20Reference) (Distance :type Float%20%28single-precision%29))
  (Transformation|SetActorTransform (Math|Transform|MakeTransform (+ (Transformation|GetActorLocation EnemyTarget) (* (Transformation|GetActorForwardVector EnemyTarget) (* -1 Distance))) (Transformation|GetActorRotation EnemyTarget) (Transformation|GetActorScale3D))))