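; BP_MovingLight is an actor that moves a spot light from point to point along its spline in an endless loop.
; Each Tick, GotoNextLocation moves the light at constant speed (InterpSpeed) straight toward the current point's world location, without following the curve.
; Once within a small tolerance, IncrementSplineIndex advances the index, resetting to zero only after it exceeds the point count.
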(event EventTick
  (params (DeltaSeconds :type Float%20%28single-precision%29))
  (CallFunction|GotoNextLocation DeltaSeconds))

(event EventBeginPlay)

(fn ConstructionScript)

(fn GotoNextLocation
  (params (DeltaTime :type Float%20%28single-precision%29))
  (bind _spline (Variables|Default|GetSpline))
  (bind _spotlight (Variables|Default|GetSpotLight))
  (bind _currentindex (Variables|Default|GetCurrentIndex))
  (bind _interp_speed (Variables|Default|GetInterp%20Speed))
  (bind _returnvalue (Spline|GetLocationatSplinePoint _spline _currentindex "World"))
  (bind _returnvalue_2 (Transformation|GetWorldLocation _spotlight))
  (bind _returnvalue_3 (Math|Interpolation|VInterptoConstant _returnvalue_2 _returnvalue DeltaTime _interp_speed))
  (Transformation|SetWorldLocation (Variables|Default|GetSpotLight) _returnvalue_3 false false)
  (if (Math|Vector|Equal(Vector) _returnvalue _returnvalue_3 25.0)
    (CallFunction|IncrementSplineIndex)))

(fn IncrementSplineIndex
  (Math|Integer|IncrementInt (Variables|Default|GetCurrentIndex)
    (:%20%20
      (if (> (Variables|Default|GetCurrentIndex) (Spline|GetNumberOfSplinePoints (Variables|Default|GetSpline)))
        (Variables|Default|SetCurrentIndex 0)))))