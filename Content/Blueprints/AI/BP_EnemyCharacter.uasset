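; BP_EnemyCharacter is an AI enemy character that displays its awareness state and alertness level on two world-space texts.
; Every tick it reads the EnemyState blackboard enum and shows it as an ellipsis, question mark or exclamation mark.
; The second text shows the rounded Alertness value from BP_EnemyController.
; Both texts rotate toward the player's camera like billboards, using a look-at rotation calculated from the state text's location.
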(event EventTick
  (params (DeltaSeconds :type Float%20%28single-precision%29))
  (bind _enemystate (Variables|Default|GetEnemyState))
  (Rendering|Components|TextRender|SetText _enemystate (Utilities|Select :Index (Utilities|Enum|ByteToEnumEEnemyState (Class|BlackboardComponent|GetValueasEnum (AI|GetBlackboard 0) (Utilities|Name|MakeLiteralName "EnemyState"))) :Idle (Utilities|Text|MakeLiteralText "...") :Searching (Utilities|Text|MakeLiteralText "?") :Pursuing (Utilities|Text|MakeLiteralText "!")))
  (Transformation|SetWorldRotation _enemystate (Math|Rotator|FindLookatRotation (Transformation|GetWorldLocation (Variables|Default|GetEnemyState)) (Transformation|GetWorldLocation (Actor|GetComponentbyClass (Game|GetPlayerCharacter 0) "/Script/Engine.CameraComponent"))) false false)
  (bind _asbp_enemy_controller (Utilities|Casting|CastToBP_EnemyController (Pawn|GetController)))
  (Rendering|Components|TextRender|SetText (Variables|Default|GetEnemyState1) (Utilities|Text|ToText(Integer) (Math|Float|Round (Variables|/Script/ProjectLigma.EnemyController|GetAlertness _asbp_enemy_controller)))))

(fn ConstructionScript)