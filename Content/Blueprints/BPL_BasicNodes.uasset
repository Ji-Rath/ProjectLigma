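; BPL_BasicNodes is a Blueprint function library with a helper that finds the world position under the mouse cursor.
; FindMousePosition checks that the target controller and its controlled pawn are valid, then deprojects the mouse into world space.
; It line-traces the Visibility channel a fixed distance along that direction and returns the impact point, without checking whether the trace hit.
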(fn FindMousePosition
  (params (Target :type Player%20Controller%20Object%20Reference))
  (bind (_worldlocation _worlddirection _returnvalue) (Game|Player|ConvertMouseLocationToWorldSpace Target))
  (Utilities|IsValid Target
    (:Is%20Valid
      (if (and (Utilities|IsValid (Pawn|GetControlledPawn Target)) _returnvalue)
        (bind _outhit (Collision|LineTraceByChannel 0 _worldlocation (+ _worldlocation (* _worlddirection 5e+03)) "TraceTypeQuery1" false 0 "None"))
        (return (.ImpactPoint (Collision|BreakHitResult _outhit)))))))